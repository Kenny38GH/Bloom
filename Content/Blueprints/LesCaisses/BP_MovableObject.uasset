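; Movable crate that BP_Hero pushes or pulls along the X axis while grabbing inside its Box overlap.
; Each Tick, it line-traces down from the player-side edge against every BP_Floor, toggling physics off on a hit and on for a miss.
; On a hit, a grabbed crate snaps to a fixed X offset from the hero, slows their walk speed and ignores BP_Trigger_Room1 when moving.
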(event `self.ReceiveBeginPlay`
  (bind _asbp_hero (cast `/Game/Blueprints/Hero/BP_Hero` (`GameplayStatics.GetPlayerCharacter` 0)))
  (set `self.PlayerRef` _asbp_hero)
  (bind _outactors (`GameplayStatics.GetAllActorsOfClass` "/Game/Blueprints/LesCaisses/BP_Floor.BP_Floor_C"))
  (set `self.FloorsRef` _outactors)
  (bind _returnvalue (`GameplayStatics.GetActorOfClass` "/Game/Blueprints/Triggers_Room/BP_Trigger_Room1.BP_Trigger_Room1_C"))
  (set `self.TriggerRoom1Ref` _returnvalue)
  (`PrimitiveComponent.SetSimulatePhysics` (`self.Move`) false))

(event `self.Box.OnComponentBeginOverlap`
  (params (OverlappedComponent :type "PrimitiveComponent Object Reference") (OtherActor :type "Actor Object Reference") (OtherComp :type "PrimitiveComponent Object Reference") (OtherBodyIndex :type Integer) (bFromSweep :type Boolean) (SweepResult :type "HitResult Structure (by ref)"))
  (if (== OtherActor (`self.PlayerRef`))
    (set `self.IsBeingOverlap` true)
    (else
      (set `self.IsBeingOverlap` false))))

(event `self.Box.OnComponentEndOverlap`
  (params (OverlappedComponent :type "PrimitiveComponent Object Reference") (OtherActor :type "Actor Object Reference") (OtherComp :type "PrimitiveComponent Object Reference") (OtherBodyIndex :type Integer))
  (if (== OtherActor (`self.PlayerRef`))
    (set `self.IsBeingOverlap` false)
    (set `CharacterMovementComponent.MaxWalkSpeed` 600.0 (`Character.CharacterMovement` (`self.PlayerRef`)))))

(event `self.ReceiveTick`
  (params (DeltaSeconds :type "Float (single-precision)"))
  (bind _move (`self.Move`))
  (bind _playerref (`self.PlayerRef`))
  (bind _playerref_2 (`self.PlayerRef`))
  (bind _move_2 (`self.Move`))
  (bind (_returnvalue_x _returnvalue_y _returnvalue_z) (`KismetMathLibrary.BreakVector` (`SceneComponent.K2_GetComponentLocation` (`self.Move`))))
  (bind _returnvalue_x_2 (`KismetMathLibrary.BreakVector` (`self.K2_GetActorLocation` (`self.PlayerRef`))))
  (bind (_returnvalue_x_3 _returnvalue_y_2 _returnvalue_z_2) (`KismetMathLibrary.BreakVector` (`SceneComponent.K2_GetComponentLocation` (`self.Move`))))
  (bind _returnvalue_x_4 (`KismetMathLibrary.BreakVector` (`SceneComponent.K2_GetComponentLocation` (`self.Move`))))
  (bind _returnvalue_x_5 (`KismetMathLibrary.BreakVector` (`self.K2_GetActorLocation` (`self.PlayerRef`))))
  (bind (_returnvalue_x_6 _returnvalue_y_3 _returnvalue_z_3) (`KismetMathLibrary.BreakVector` (`SceneComponent.K2_GetComponentLocation` (`self.Move`))))
  (bind _returnvalue_x_7 (`KismetMathLibrary.BreakVector` (`self.K2_GetActorLocation` (`self.PlayerRef`))))
  (bind (_returnvalue_x_8 _returnvalue_y_4 _returnvalue_z_4) (`KismetMathLibrary.BreakVector` (`SceneComponent.K2_GetComponentLocation` (`self.Move`))))
  (bind _returnvalue_x_9 (`KismetMathLibrary.BreakVector` (`SceneComponent.K2_GetComponentLocation` (`self.Move`))))
  (bind _returnvalue_x_10 (`KismetMathLibrary.BreakVector` (`self.K2_GetActorLocation` (`self.PlayerRef`))))
  (bind (_returnvalue_x_11 _returnvalue_y_5 _returnvalue_z_5) (`KismetMathLibrary.BreakVector` (`SceneComponent.K2_GetComponentLocation` (`self.Move`))))
  (bind (_returnvalue_x_12 _returnvalue_y_6 _returnvalue_z_6) (`KismetMathLibrary.BreakVector` (`SceneComponent.K2_GetComponentLocation` (`self.Move`))))
  (bind _returnvalue_x_13 (`KismetMathLibrary.BreakVector` (`SceneComponent.K2_GetComponentLocation` (`self.Move`))))
  (bind _charactermovement (`Character.CharacterMovement` _playerref_2))
  (bind _charactermovement_2 (`Character.CharacterMovement` _playerref))
  (bind _returnvalue_x_14 (`KismetMathLibrary.BreakVector` (`SceneComponent.K2_GetComponentLocation` (`Actor.RootComponent` (`self.PlayerRef`)))))
  (bind _returnvalue_x_15 (`KismetMathLibrary.BreakVector` (`SceneComponent.K2_GetComponentLocation` (`Actor.RootComponent` (`self.PlayerRef`)))))
  (bind _returnvalue_x_16 (`KismetMathLibrary.BreakVector` (`SceneComponent.K2_GetComponentLocation` (`Actor.RootComponent` (`self.PlayerRef`)))))
  (bind _returnvalue (+ _returnvalue_x_12 -100.0))
  (bind _returnvalue_2 (+ _returnvalue_x 100.0))
  (if (> (- _returnvalue_x_9 _returnvalue_x_15) 0.0)
    (for _array_element (`self.FloorsRef`)
      (bind (_hitlocation _hitnormal _bonename _outhit _returnvalue_3) (`PrimitiveComponent.K2_LineTraceComponent` (`/Game/Blueprints/LesCaisses/BP_Floor.Floor` _array_element) (`KismetMathLibrary.MakeVector` _returnvalue _returnvalue_y_6 _returnvalue_z_6) (`KismetMathLibrary.MakeVector` _returnvalue _returnvalue_y_6 (- _returnvalue_z_6 (`self.DetectionZoneFloor`))) false false false))
      (if _returnvalue_3
        (`PrimitiveComponent.SetSimulatePhysics` _move false)
        (if (`self.IsBeingOverlap`)
          (if (`/Game/Blueprints/Hero/BP_Hero.IsGrabing` (`self.PlayerRef`))
            (set `/Game/Blueprints/Hero/BP_Hero.IsPushing` true _playerref_2)
            (set `CharacterMovementComponent.MaxWalkSpeed` 200.0 _charactermovement)
            (`PrimitiveComponent.IgnoreActorWhenMoving` (`self.Move`) (`self.TriggerRoom1Ref`) true)
            ;[1 1 1] PULL&PUSH
            (if (> (- _returnvalue_x_13 _returnvalue_x_16) 0.0)
              ;;[1 1 1] Quand Player est à gauche
              (`self.K2_SetActorLocation` (`KismetMathLibrary.MakeVector` (+ _returnvalue_x_7 140.0) _returnvalue_y_4 _returnvalue_z_4))
              (else
                ;;[1 1 1] Quand Player est à droite
                (`self.K2_SetActorLocation` (`KismetMathLibrary.MakeVector` (+ _returnvalue_x_10 -140.0) _returnvalue_y_5 _returnvalue_z_5))))
            (else
              (set `/Game/Blueprints/Hero/BP_Hero.IsPushing` false _playerref_2)
              (set `CharacterMovementComponent.MaxWalkSpeed` 600.0 _charactermovement))))
        (else
          (`PrimitiveComponent.SetSimulatePhysics` _move true))))
    (else
      (for _array_element_2 (`self.FloorsRef`)
        (bind (_hitlocation_2 _hitnormal_2 _bonename_2 _outhit_2 _returnvalue_4) (`PrimitiveComponent.K2_LineTraceComponent` (`/Game/Blueprints/LesCaisses/BP_Floor.Floor` _array_element_2) (`KismetMathLibrary.MakeVector` _returnvalue_2 _returnvalue_y _returnvalue_z) (`KismetMathLibrary.MakeVector` _returnvalue_2 _returnvalue_y (- _returnvalue_z (`self.DetectionZoneFloor`))) false false false))
        (if _returnvalue_4
          (`PrimitiveComponent.SetSimulatePhysics` _move_2 false)
          (if (`self.IsBeingOverlap`)
            (if (`/Game/Blueprints/Hero/BP_Hero.IsGrabing` (`self.PlayerRef`))
              (set `/Game/Blueprints/Hero/BP_Hero.IsPushing` true _playerref)
              (set `CharacterMovementComponent.MaxWalkSpeed` 200.0 _charactermovement_2)
              (`PrimitiveComponent.IgnoreActorWhenMoving` (`self.Move`) (`self.TriggerRoom1Ref`) true)
              ;[1 1 1] PULL&PUSH
              (if (> (- _returnvalue_x_4 _returnvalue_x_14) 0.0)
                ;;[1 1 1] Quand Player est à gauche
                (`self.K2_SetActorLocation` (`KismetMathLibrary.MakeVector` (+ _returnvalue_x_2 140.0) _returnvalue_y_2 _returnvalue_z_2))
                (else
                  ;;[1 1 1] Quand Player est à droite
                  (`self.K2_SetActorLocation` (`KismetMathLibrary.MakeVector` (+ _returnvalue_x_5 -140.0) _returnvalue_y_3 _returnvalue_z_3))))
              (else
                (set `/Game/Blueprints/Hero/BP_Hero.IsPushing` false _playerref)
                (set `CharacterMovementComponent.MaxWalkSpeed` 600.0 _charactermovement_2))))
          (else
            (`PrimitiveComponent.SetSimulatePhysics` _move_2 true)))))))

(fn `UserConstructionScript`)