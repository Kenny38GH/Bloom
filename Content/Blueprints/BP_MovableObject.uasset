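; BP_MovableObject is an object that BP_Hero can push or pull along the X axis by grabbing it.
; A Box overlap flags when the player is in range, and Tick checks the hero's grab state.
; While grabbed, it lowers its mass, slows the hero and snaps to a fixed X offset on its current side.
; Releasing restores walk speed and raises mass, while leaving the Box only restores speed.
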(event `self.ReceiveBeginPlay`
  (bind _asbp_hero (cast `/Game/Blueprints/Hero/BP_Hero` (`GameplayStatics.GetPlayerCharacter` 0)))
  (set `self.PlayerRef` _asbp_hero))

(event `self.Box.OnComponentBeginOverlap`
  (params (OverlappedComponent :type "PrimitiveComponent Object Reference") (OtherActor :type "Actor Object Reference") (OtherComp :type "PrimitiveComponent Object Reference") (OtherBodyIndex :type Integer) (bFromSweep :type Boolean) (SweepResult :type "HitResult Structure (by ref)"))
  (if (== OtherActor (`self.PlayerRef`))
    (set `self.IsBeingOverlap` true)
    (else
      (set `self.IsBeingOverlap` false))))

(event `self.Box.OnComponentEndOverlap`
  (params (OverlappedComponent :type "PrimitiveComponent Object Reference") (OtherActor :type "Actor Object Reference") (OtherComp :type "PrimitiveComponent Object Reference") (OtherBodyIndex :type Integer))
  (if (== OtherActor (`self.PlayerRef`))
    (set `self.IsBeingOverlap` false)
    (set `CharacterMovementComponent.MaxWalkSpeed` 600.0 (`Character.CharacterMovement` (`self.PlayerRef`)))))

(event `self.ReceiveTick`
  (params (DeltaSeconds :type "Float (single-precision)"))
  (bind _playerref (`self.PlayerRef`))
  (bind _returnvalue_x (`KismetMathLibrary.BreakVector` (`SceneComponent.K2_GetComponentLocation` (`self.Move`))))
  (bind _returnvalue_x_2 (`KismetMathLibrary.BreakVector` (`self.K2_GetActorLocation` (`self.PlayerRef`))))
  (bind (_returnvalue_x_3 _returnvalue_y _returnvalue_z) (`KismetMathLibrary.BreakVector` (`SceneComponent.K2_GetComponentLocation` (`self.Move`))))
  (bind _returnvalue_x_4 (`KismetMathLibrary.BreakVector` (`self.K2_GetActorLocation` (`self.PlayerRef`))))
  (bind (_returnvalue_x_5 _returnvalue_y_2 _returnvalue_z_2) (`KismetMathLibrary.BreakVector` (`SceneComponent.K2_GetComponentLocation` (`self.Move`))))
  (bind _charactermovement (`Character.CharacterMovement` _playerref))
  (bind _returnvalue_x_6 (`KismetMathLibrary.BreakVector` (`SceneComponent.K2_GetComponentLocation` (`Actor.RootComponent` (`self.PlayerRef`)))))
  (if (`self.IsBeingOverlap`)
    (if (`/Game/Blueprints/Hero/BP_Hero.IsGrabing` (`self.PlayerRef`))
      (set `/Game/Blueprints/Hero/BP_Hero.IsPushing` true _playerref)
      (set `CharacterMovementComponent.MaxWalkSpeed` 200.0 _charactermovement)
      (`PrimitiveComponent.SetMassOverrideInKg` (`self.Move`) "None" 100.0 true)
      (if (> (- _returnvalue_x _returnvalue_x_6) 0.0)
        ;[1 1 1] Tirer/Pousser Quand Player est à gauche
        (`self.K2_SetActorLocation` (`KismetMathLibrary.MakeVector` (+ _returnvalue_x_2 130.0) _returnvalue_y _returnvalue_z))
        (else
          ;[1 1 1] Tirer/Pousser Quand Player est à droite
          (`self.K2_SetActorLocation` (`KismetMathLibrary.MakeVector` (+ _returnvalue_x_4 -130.0) _returnvalue_y_2 _returnvalue_z_2))))
      (else
        (set `/Game/Blueprints/Hero/BP_Hero.IsPushing` false _playerref)
        (set `CharacterMovementComponent.MaxWalkSpeed` 600.0 _charactermovement)
        (`PrimitiveComponent.SetMassOverrideInKg` (`self.Move`) "None" 1000.0 true)))))

(fn `UserConstructionScript`)