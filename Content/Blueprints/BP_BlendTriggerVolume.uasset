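; Trigger volume that switches the player's view to a static camera while BP_Hero is inside it.
; On begin overlap, the hero's PlayerController blends its view target to the first actor found of the StaticCamera class.
; On end overlap, it blends back to the hero, with both transitions timed by CameraBlendTime.
; The camera is looked up by class on each entry rather than through an instance reference.
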(event `self.OverlapVolume.OnComponentBeginOverlap`
  (params (OverlappedComponent :type "PrimitiveComponent Object Reference") (OtherActor :type "Actor Object Reference") (OtherComp :type "PrimitiveComponent Object Reference") (OtherBodyIndex :type Integer) (bFromSweep :type Boolean) (SweepResult :type "HitResult Structure (by ref)"))
  (bind _asbp_hero (cast `/Game/Blueprints/Hero/BP_Hero` OtherActor))
  (if (`KismetSystemLibrary.IsValid` _asbp_hero)
    (bind _asplayer_controller (cast `PlayerController` (`Pawn.GetController` _asbp_hero)))
    (if (`KismetSystemLibrary.IsValid` _asplayer_controller)
      (bind _returnvalue (`GameplayStatics.GetActorOfClass` "/Game/Blueprints/StaticCamera.StaticCamera_C"))
      (`PlayerController.SetViewTargetWithBlend` _asplayer_controller _returnvalue (`self.CameraBlendTime`) "VTBlend_Linear" 0.0 false))))

(event `self.OverlapVolume.OnComponentEndOverlap`
  (params (OverlappedComponent :type "PrimitiveComponent Object Reference") (OtherActor :type "Actor Object Reference") (OtherComp :type "PrimitiveComponent Object Reference") (OtherBodyIndex :type Integer))
  (bind _asbp_hero (cast `/Game/Blueprints/Hero/BP_Hero` OtherActor))
  (if (`KismetSystemLibrary.IsValid` _asbp_hero)
    (bind _asplayer_controller (cast `PlayerController` (`Pawn.GetController` _asbp_hero)))
    (if (`KismetSystemLibrary.IsValid` _asplayer_controller)
      (`PlayerController.SetViewTargetWithBlend` _asplayer_controller _asbp_hero (`self.CameraBlendTime`) "VTBlend_Linear" 0.0 false))))

(fn `UserConstructionScript`)