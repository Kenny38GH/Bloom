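; BP_Hero is the player character for a sprite-based side-scroller, moving along X and turning to face its velocity unless movement is locked.
; Jump in midair runs an enlarged capsule trace to wall-jump off the hit normal, falling back to a normal Jump.
; Launch, jump and ledge events switch the animation state machine to Airborne unless Grab is held.
; SpawnDust places a landing dust effect at the sprite.
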(event `InputAction|Grab`
  (params (Key :type "Key Structure"))
  (:`Pressed`
    (set `self.IsGrabing` true))
  (:`Released`
    (set `self.IsGrabing` false)))

(event `InputAxis|Forward`
  (params (AxisValue :type "Float (single-precision)"))
  (if (not (`self.IsMovementLoked`))
    (`self.AddMovementInput` (1.0 0.0 0.0) AxisValue)))

(event `self.OnLaunched`
  (params (LaunchVelocity :type "Vector Structure") (bXYOverride :type Boolean) (bZOverride :type Boolean))
  (if (not (`self.IsGrabing`)) :!label _label
    (`PaperZDAnimInstance.JumpToNode` (`PaperZDAnimationComponent.AnimInstance` (`self.AnimationComponent`)) "Airborne" "None")))

(event `self.OnJumped`
  (goto _label))

(event `self.OnWalkingOffLedge`
  (params (PreviousFloorImpactNormal :type "Vector Structure (by ref)") (PreviousFloorContactNormal :type "Vector Structure (by ref)") (PreviousLocation :type "Vector Structure (by ref)") (TimeDelta :type "Float (single-precision)"))
  (goto _label))

(event `InputAction|Jump`
  (params (Key :type "Key Structure"))
  (bind _returnvalue (`self.K2_GetActorLocation`))
  (bind _capsulecomponent (`self.CapsuleComponent`))
  (:`Pressed`
    (if (`NavMovementComponent.IsMovingOnGround` (`self.CharacterMovement`))
      (`self.Jump` :!label _label_2)
      (else
        (bind (_outhit _returnvalue_2) (`KismetSystemLibrary.CapsuleTraceSingle` _returnvalue _returnvalue (+ (`CapsuleComponent.CapsuleRadius` _capsulecomponent) 10.0) (`CapsuleComponent.CapsuleHalfHeight` _capsulecomponent) "TraceTypeQuery2"))
        (if _returnvalue_2
          (`self.LaunchCharacter` (`KismetMathLibrary.MakeVector` (.x (* (`.Normal` (`GameplayStatics.BreakHitResult` _outhit)) (60.0 60.0 60.0))) (.y (* (`.Normal` (`GameplayStatics.BreakHitResult` _outhit)) (60.0 60.0 60.0))) (+ (.z (* (`.Normal` (`GameplayStatics.BreakHitResult` _outhit)) (60.0 60.0 60.0))) (`CharacterMovementComponent.JumpZVelocity` (`self.CharacterMovement`)))) false true)
          (else
            (goto _label_2))))))
  (:`Released`
    (`self.StopJumping`)))

(event `self.ReceiveTick`
  (params (DeltaSeconds :type "Float (single-precision)"))
  (bind _returnvalue (`self.GetController`))
  (bind _returnvalue_2 (`self.GetController`))
  (`parent.ReceiveTick` DeltaSeconds)
  (if (not (`self.IsMovementLoked`))
    (`/Engine/EditorBlueprintResources/StandardMacros.CompareFloat` (.x (`MovementComponent.Velocity` (`self.GetMovementComponent`)))
      (:`>`
        ;[0 0.4745 1] Look Right
        (`/Engine/EditorBlueprintResources/StandardMacros.IsValid` _returnvalue_2
          (:`Is Valid`
            (`Controller.SetControlRotation` _returnvalue_2 (`KismetMathLibrary.MakeRotator` 0.0)))))
      (:`<`
        ;[0 0.4745 1] Look Left
        (`/Engine/EditorBlueprintResources/StandardMacros.IsValid` _returnvalue
          (:`Is Valid`
            (`Controller.SetControlRotation` _returnvalue (`KismetMathLibrary.MakeRotator` 0.0 0.0 180.0))))))))

(fn `SpawnDust`
  (bind (_returnvalue_location _returnvalue_rotation) (`KismetMathLibrary.BreakTransform` (`SceneComponent.K2_GetComponentToWorld` (`self.Sprite`))))
  (`|SpawnActorFromClass` "/Game/Blueprints/Hero/BP_LandDust.BP_LandDust_C" (`KismetMathLibrary.MakeTransform` _returnvalue_location _returnvalue_rotation) "Undefined" "OverrideRootScale" null null))

(fn `UserConstructionScript`)