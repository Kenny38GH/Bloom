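; BP_LanternToActivate is a lantern whose point light fades in and out when activated or deactivated.
; It starts dark, and the ActivateLight and DesactivateLight events only toggle an IsLightOn flag.
; Tick uses FInterpTo to ease the light intensity toward a fixed target when on, or back toward zero when off, at the InterpSpeed rate.
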(event `self.ReceiveBeginPlay`
  (`LightComponent.SetIntensity` (`self.PointLight`) 0.0)
  (set `self.IntensityToReach` 5338.0)
  (set `self.IsLightOn` false))

(event `ActivateLight`
  (set `self.IsLightOn` true))

(event `DesactivateLight`
  (set `self.IsLightOn` false))

(event `self.ReceiveTick`
  (params (DeltaSeconds :type "Float (single-precision)"))
  (bind _pointlight (`self.PointLight`))
  (bind _pointlight_2 (`self.PointLight`))
  (bind _interp_speed (`self.Interp Speed`))
  (if (`self.IsLightOn`)
    (`LightComponent.SetIntensity` _pointlight_2 (`KismetMathLibrary.FInterpTo` (`LightComponentBase.Intensity` _pointlight_2) (`self.IntensityToReach`) DeltaSeconds _interp_speed))
    (elif (> (`LightComponentBase.Intensity` (`self.PointLight`)) 0.0)
      (`LightComponent.SetIntensity` _pointlight (`KismetMathLibrary.FInterpTo` (`LightComponentBase.Intensity` _pointlight) 0.0 DeltaSeconds _interp_speed)))))

(fn `UserConstructionScript`)