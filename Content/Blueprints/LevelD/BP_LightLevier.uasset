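; BP_LightLevier is a lever the hero can toggle to switch a linked lantern and door on or off.
; Overlapping its Box with BP_Hero enables player input on the lever, and leaving disables it.
; The Activate action checks the lantern's IsLightOn state, then calls the matching activate or deactivate functions on both targets.
; A timeline plays forward or in reverse to animate the lever's pitch.
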(event `self.Box.OnComponentBeginOverlap`
  (params (OverlappedComponent :type "PrimitiveComponent Object Reference") (OtherActor :type "Actor Object Reference") (OtherComp :type "PrimitiveComponent Object Reference") (OtherBodyIndex :type Integer) (bFromSweep :type Boolean) (SweepResult :type "HitResult Structure (by ref)"))
  (cast `/Game/Blueprints/Hero/BP_Hero` OtherActor)
  (`self.EnableInput` (`GameplayStatics.GetPlayerController` 0)))

(event `self.Box.OnComponentEndOverlap`
  (params (OverlappedComponent :type "PrimitiveComponent Object Reference") (OtherActor :type "Actor Object Reference") (OtherComp :type "PrimitiveComponent Object Reference") (OtherBodyIndex :type Integer))
  (cast `/Game/Blueprints/Hero/BP_Hero` OtherActor)
  (`self.DisableInput` (`GameplayStatics.GetPlayerController` 0)))

(event `InputAction|Activate`
  (params (Key :type "Key Structure"))
  (bind _doortoactivate (`self.DoorToActivate`))
  (bind _lanterntoactivate (`self.LanternToActivate`))
  (:`Pressed`
    (if (`/Game/Blueprints/LevelD/BP_LanternToActivate.IsLightOn` (`self.LanternToActivate`))
      (`/Game/Blueprints/LevelD/BP_LanternToActivate.DesactivateLight` _lanterntoactivate)
      (`/Game/Blueprints/LevelD/BP_DoorLevier.SwitchDeactivated` _doortoactivate)
      (bind (_direction _newtrack_0) (`Timeline|Timeline_1` :!via `Reverse` :!label _label)
        (:`Update`
          (`SceneComponent.K2_SetRelativeRotation` (`self.Levier`) (`KismetMathLibrary.MakeRotator` 0.0 _newtrack_0) false false)))
      (else
        (`/Game/Blueprints/LevelD/BP_LanternToActivate.ActivateLight` _lanterntoactivate)
        (`/Game/Blueprints/LevelD/BP_DoorLevier.SwitchActivated` _doortoactivate)
        (goto _label)))))

(fn `UserConstructionScript`)