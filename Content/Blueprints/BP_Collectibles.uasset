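; BP_Collectibles is a pickup actor that the player collects by pressing E while standing in its box.
; Box overlaps with BP_Hero enable input on the actor for player controller 0, and end overlaps disable it.
; On E, it decrements CollectiblesLeft on GM_Base, adds a new BP_Collectibles_Widget to the viewport and destroys itself.
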(event `Key|E`
  (params (Key :type "Key Structure"))
  (:`Pressed`
    (bind _asgm_base (cast `/Game/Blueprints/GM_Base` (`GameplayStatics.GetGameMode`)))
    (bind _result (`/Engine/EditorBlueprintResources/StandardMacros.DecrementInt` (`/Game/Blueprints/GM_Base.Collectibles left` _asgm_base))
      (:`  `
        (set `/Game/Blueprints/GM_Base.Collectibles left` _result _asgm_base)
        (bind _returnvalue (`|CreateWidget` "/Game/UserInterface/BP_Collectibles_Widget.BP_Collectibles_Widget_C"))
        (`UserWidget.AddToViewport` _returnvalue 0)
        (`self.K2_DestroyActor`)))))

(event `self.Box.OnComponentBeginOverlap`
  (params (OverlappedComponent :type "PrimitiveComponent Object Reference") (OtherActor :type "Actor Object Reference") (OtherComp :type "PrimitiveComponent Object Reference") (OtherBodyIndex :type Integer) (bFromSweep :type Boolean) (SweepResult :type "HitResult Structure (by ref)"))
  (cast `/Game/Blueprints/Hero/BP_Hero` OtherActor)
  (`self.EnableInput` (`GameplayStatics.GetPlayerController` 0)))

(event `self.Box.OnComponentEndOverlap`
  (params (OverlappedComponent :type "PrimitiveComponent Object Reference") (OtherActor :type "Actor Object Reference") (OtherComp :type "PrimitiveComponent Object Reference") (OtherBodyIndex :type Integer))
  (cast `/Game/Blueprints/Hero/BP_Hero` OtherActor)
  (`self.DisableInput` (`GameplayStatics.GetPlayerController` 0)))

(fn `UserConstructionScript`)