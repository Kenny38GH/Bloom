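; Player-controlled camera arm actor that pans freely through the world, apparently for a mapping view.
; BeginPlay enables input from the first player controller and stores the root's starting location.
; Axis inputs shift the root along world X, Y and Z by a fixed step per tick, without delta-time scaling.
; The Camera Default Loc action snaps it back to the stored start location.
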(event `InputAction|Camera Default Loc`
  (params (Key :type "Key Structure"))
  (:`Pressed`
    (`SceneComponent.K2_SetWorldLocation` (`self.DefaultSceneRoot`) (`self.DefaultLoc`) false false)))

(event `self.ReceiveBeginPlay`
  (`self.EnableInput` (`GameplayStatics.GetPlayerController` 0))
  (set `self.DefaultLoc` (`SceneComponent.K2_GetComponentLocation` (`self.DefaultSceneRoot`))))

(event `InputAxis|Camera Up`
  (params (AxisValue :type "Float (single-precision)"))
  (bind (_returnvalue_x _returnvalue_y _returnvalue_z) (`KismetMathLibrary.BreakVector` (`SceneComponent.K2_GetComponentLocation` (`self.DefaultSceneRoot`))))
  (if (> AxisValue 0.0)
    (`SceneComponent.K2_SetWorldLocation` (`self.DefaultSceneRoot`) (`KismetMathLibrary.MakeVector` _returnvalue_x _returnvalue_y (+ _returnvalue_z (* AxisValue 10.0))) false false)))

(event `InputAxis|Camera Down`
  (params (AxisValue :type "Float (single-precision)"))
  (bind (_returnvalue_x _returnvalue_y _returnvalue_z) (`KismetMathLibrary.BreakVector` (`SceneComponent.K2_GetComponentLocation` (`self.DefaultSceneRoot`))))
  (if (> AxisValue 0.0)
    (`SceneComponent.K2_SetWorldLocation` (`self.DefaultSceneRoot`) (`KismetMathLibrary.MakeVector` _returnvalue_x _returnvalue_y (- _returnvalue_z (* AxisValue 10.0))) false false)))

(event `InputAxis|Camera L/R`
  (params (AxisValue :type "Float (single-precision)"))
  (bind (_returnvalue_x _returnvalue_y _returnvalue_z) (`KismetMathLibrary.BreakVector` (`SceneComponent.K2_GetComponentLocation` (`self.DefaultSceneRoot`))))
  (`SceneComponent.K2_SetWorldLocation` (`self.DefaultSceneRoot`) (`KismetMathLibrary.MakeVector` (+ _returnvalue_x (* AxisValue 10.0)) _returnvalue_y _returnvalue_z) false false))

(event `InputAxis|Camera Y`
  (params (AxisValue :type "Float (single-precision)"))
  (bind (_returnvalue_x _returnvalue_y _returnvalue_z) (`KismetMathLibrary.BreakVector` (`SceneComponent.K2_GetComponentLocation` (`self.DefaultSceneRoot`))))
  (`SceneComponent.K2_SetWorldLocation` (`self.DefaultSceneRoot`) (`KismetMathLibrary.MakeVector` _returnvalue_x (+ _returnvalue_y (* AxisValue 10.0)) _returnvalue_z) false false))

(fn `UserConstructionScript`)