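; BP_PlateformUpDown is a moving platform, up and down by its name, that stays still until a lever flag turns on.
; An InterpToMovement component drives the motion and is stopped at BeginPlay.
; Tick polls LevierOn on the GM_Base game mode, then restarts the movement and latches IsMoving.
; Once moving, Tick calls Activate on the component each frame and never rechecks the lever.
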(event `self.ReceiveBeginPlay`
  (`MovementComponent.StopMovementImmediately` (`self.InterpToMovement`))
  (set `self.IsMoving` false))

(event `self.ReceiveTick`
  (params (DeltaSeconds :type "Float (single-precision)"))
  (if (`self.IsMoving`)
    (`ActorComponent.Activate` (`self.InterpToMovement`) false)
    (else
      (bind _asgm_base (cast `/Game/Blueprints/GM_Base` (`GameplayStatics.GetGameMode`)))
      (if (`/Game/Blueprints/GM_Base.LevierOn` _asgm_base)
        (`InterpToMovementComponent.RestartMovement` (`self.InterpToMovement`) 1.0)
        (set `self.IsMoving` true)))))

(fn `UserConstructionScript`)