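; PaperZD-style animation notify, shown as "Land", that handles the hero's landing impact.
; On notify, it spawns dust on BP_Hero, then runs a sphere overlap at an offset from the sprite, with offset and radius scaled by the sprite's X scale.
; Other Characters caught in the sphere are launched upward.
; Without a valid owning instance, it draws a debug sphere of the hit area instead.
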(event `self.OnReceiveNotify`
  (params (OwningInstance :type "PaperZDAnimInstance Object Reference"))
  (`/Engine/EditorBlueprintResources/StandardMacros.IsValid` OwningInstance
    (:`Is Valid`
      (bind _asbp_hero (cast `/Game/Blueprints/Hero/BP_Hero` (`PaperZDAnimInstance.PaperCharacter` OwningInstance)))
      (`/Game/Blueprints/Hero/BP_Hero.SpawnDust` _asbp_hero)
      (bind _sprite (`PaperCharacter.Sprite` _asbp_hero))
      (bind _relativescale3d_x (`KismetMathLibrary.BreakVector` (`SceneComponent.RelativeScale3D` _sprite)))
      (bind _outactors (`KismetSystemLibrary.SphereOverlapActors` (+ (* (`self.Position`) _relativescale3d_x) (`SceneComponent.K2_GetComponentLocation` _sprite)) (* _relativescale3d_x (`self.Radius`)) (`|MakeArray` "ObjectTypeQuery3" "ObjectTypeQuery4" :!type "EObjectTypeQuery Enum") "/Script/Engine.Character" (`|MakeArray` _asbp_hero :!type "Actor Object Reference")))
      (for _array_element _outactors
        (bind _ascharacter (cast `Character` _array_element))
        (`Character.LaunchCharacter` _ascharacter (* (`KismetMathLibrary.Vector_Up`) 750.0) false false)))
    (:`Is Not Valid`
      (`KismetSystemLibrary.DrawDebugSphere` (`self.Position`) (`self.Radius`) 12 (struct :`R` 1.0 :`G` 1.0 :`B` 1.0 :`A` 1.0) 0.1 0.1))))

(fn `GetDisplayName`
  (returns (ReturnValue :type Name))
  (return "Land"))