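; BP_Trigger_Room4 is a trigger volume that fades the outside of Room 4 out while the player hero is inside it.
; Box overlap events set a target opacity to zero when the hero enters and one when it leaves; any other actor entering also resets it to one.
; Tick smoothly interpolates the GlobalOpacityPower scalar in the MPC_OutsideRoom4 material parameter collection toward that target.
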(event `self.ReceiveBeginPlay`
  (bind _asbp_hero (cast `/Game/Blueprints/Hero/BP_Hero` (`GameplayStatics.GetPlayerCharacter` 0)))
  (set `self.PlayerRef` _asbp_hero)
  (set `self.OpacityValue` 1.0))

(event `self.Box.OnComponentBeginOverlap`
  (params (OverlappedComponent :type "PrimitiveComponent Object Reference") (OtherActor :type "Actor Object Reference") (OtherComp :type "PrimitiveComponent Object Reference") (OtherBodyIndex :type Integer) (bFromSweep :type Boolean) (SweepResult :type "HitResult Structure (by ref)"))
  (if (== OtherActor (`self.PlayerRef`))
    (set `self.OpacityValue` 0.0)
    (else
      (set `self.OpacityValue` 1.0 :!label _label))))

(event `self.Box.OnComponentEndOverlap`
  (params (OverlappedComponent :type "PrimitiveComponent Object Reference") (OtherActor :type "Actor Object Reference") (OtherComp :type "PrimitiveComponent Object Reference") (OtherBodyIndex :type Integer))
  (if (== OtherActor (`self.PlayerRef`))
    (goto _label)))

(event `self.ReceiveTick`
  (params (DeltaSeconds :type "Float (single-precision)"))
  (bind _returnvalue (`KismetMaterialLibrary.GetScalarParameterValue` "/Game/Materials/Outside_Rooms/MPC_OutsideRoom4.MPC_OutsideRoom4" "GlobalOpacityPower"))
  (`KismetMaterialLibrary.SetScalarParameterValue` "/Game/Materials/Outside_Rooms/MPC_OutsideRoom4.MPC_OutsideRoom4" "GlobalOpacityPower" (`KismetMathLibrary.FInterpTo` _returnvalue (`self.OpacityValue`) DeltaSeconds 2.0)))

(fn `UserConstructionScript`)